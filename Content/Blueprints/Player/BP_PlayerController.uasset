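; Player controller that handles respawning and the hold-to-show Tab menu.
; Pressing Enter while spectating calls a server respawn event, which spawns the player through the game mode only if it allows fast respawn.
; LaunchRespawnTimer schedules that same Respawn function on a stored timer, without the fast-respawn check.
; Holding Tab shows a lazily created, reused menu widget, removed from the viewport on release.
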(event `Key|Enter`
  (params (Key :type "Key Structure"))
  (:`Pressed`
    (cast `/Game/Blueprints/Game/Spectators/BP_GameSpectator` (`self.K2_GetPawn`))
    (`self.ServerRespawn`)))

(event `ServerRespawn`
  (bind _asbp_base_game_mode (cast `/Game/Blueprints/Game/BP_BaseGameMode` (`GameplayStatics.GetGameMode`)))
  (if (`/Game/Blueprints/Game/BP_BaseGameMode.AllowFastRespawn` _asbp_base_game_mode)
    (`self.Respawn`)))

(event `Key|Tab`
  (params (Key :type "Key Structure"))
  ;[1 1 1] TabMenu
  (:`Pressed`
    (`self.ToggleTabMenu` true))
  (:`Released`
    (`self.ToggleTabMenu` false)))

(fn `LaunchRespawnTimer`
  (params (Time :type "Float (double-precision)"))
  (bind _returnvalue (`KismetSystemLibrary.K2_SetTimer` null "Respawn" Time))
  (set `self.RespawnTimer` _returnvalue))

(fn `Respawn`
  (bind _asbp_base_game_mode (cast `/Game/Blueprints/Game/BP_BaseGameMode` (`GameplayStatics.GetGameMode`)))
  (`/Game/Blueprints/Game/BP_BaseGameMode.SpawnPlayer` _asbp_base_game_mode self))

(fn `ToggleTabMenu`
  (params (Show :type Boolean))
  (if Show
    (bind _tabmenu (`self.TabMenu`)
      (:`then`
        (`UserWidget.AddToViewport` _tabmenu 0))
      (:`else`
        (bind _returnvalue (`|CreateWidget` "/Game/UI/Tabmenu/W_TabMenu.W_TabMenu_C" self))
        (bind _output_get (set `self.TabMenu` _returnvalue))
        (`UserWidget.AddToViewport` _output_get 0)))
    (else
      (`Widget.RemoveFromParent` (`self.TabMenu`)))))

(fn `UserConstructionScript`)
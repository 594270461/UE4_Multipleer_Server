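; Base game mode that runs timed rounds, handling player spawning, deaths, scoring and spectating.
; The first tick starts a delayed round and binds the game state's time-ended event; rounds spawn each player at a random free BP_GamePlayerStart.
; Deaths update kill/death counts, optionally start a respawn timer, and possess a follow spectator at the killer or a free one otherwise.
; Stopping a round moves everyone to spectators and broadcasts the end.
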(event `self.ReceiveTick`
  (params (DeltaSeconds :type "Float (single-precision)"))
  (`/Engine/EditorBlueprintResources/StandardMacros.DoOnce` false
    (:`Completed`
      (`|ExecutionSequence`
        (:`then_0`
          (`KismetSystemLibrary.Delay` 3.0)
          (`self.StartRound`))
        (:`then_1`
          ;[1 1 1] Time limit reach event
          (bind _asbp_base_game_state (cast `/Game/Blueprints/Game/BP_BaseGameState` (`GameplayStatics.GetGameState`)))
          (add `/Game/Blueprints/Game/BP_BaseGameState.TimeEnded` _asbp_base_game_state (`|CreateDelegate` :!event `TimeLimitReched`)))))))

(fn `CharacterDead`
  (params (DeadCharacter :type "/Game/Blueprints/Player/BP_PlayerCharacter Object Reference") (GetInstigator :type "/Game/Blueprints/Player/BP_PlayerController Object Reference") (DeathCausedBy :type "Actor Object Reference"))
  (`self.CharDead` DeadCharacter GetInstigator DeathCausedBy)
  (bind _asbp_player_controller (cast `/Game/Blueprints/Player/BP_PlayerController` (`Pawn.GetController` DeadCharacter)))
  (`self.UpdateDeathPoints` _asbp_player_controller GetInstigator)
  (`|ExecutionSequence`
    (:`then_0`
      (if (`self.AutoRespawn`)
        (`/Game/Blueprints/Player/BP_PlayerController.LaunchRespawnTimer` _asbp_player_controller (`self.RespawnTime`))))
    (:`then_1`
      (`self.SpawnSpectator` _asbp_player_controller GetInstigator))))

(fn `GetFreeSpawnPoints`
  (returns (FreeSpawn :type "Array of /Game/Blueprints/Game/BP_GamePlayerStart Object Reference"))
  (locals (L_FreePoints :type "Array of /Game/Blueprints/Game/BP_GamePlayerStart Object Reference"))
  (bind _outactors (`GameplayStatics.GetAllActorsOfClass` "/Game/Blueprints/Game/BP_GamePlayerStart.BP_GamePlayerStart_C"))
  (for _array_element _outactors
    (if (`/Game/Blueprints/Game/BP_GamePlayerStart.IsFree` _array_element)
      (`KismetArrayLibrary.Array_Add` (`local.L_FreePoints`) _array_element)))
  (return (`local.L_FreePoints`)))

(fn `RespawnPlayer`)

(fn `SpawnPlayer`
  (params (Player :type "/Game/Blueprints/Player/BP_PlayerController Object Reference"))
  (locals (L_PlayerStart :type "/Game/Blueprints/Game/BP_GamePlayerStart Object Reference"))
  (bind _returnvalue (`Controller.K2_GetPawn` Player))
  (`/Engine/EditorBlueprintResources/StandardMacros.IsValid` _returnvalue
    (:`Is Valid`
      (`self.K2_DestroyActor` _returnvalue))
    (:`Is Not Valid`
      _))
  (bind _freespawn (`self.GetFreeSpawnPoints`))
  (bind _output_get (set `local.L_PlayerStart` (`|GetArrayItem` _freespawn (`KismetMathLibrary.RandomInteger` (`KismetArrayLibrary.Array_LastIndex` _freespawn)))))
  (`/Game/Blueprints/Game/BP_GamePlayerStart.SpawnCharacter` _output_get Player))

(fn `SpawnSpectator`
  (params (Player :type "/Game/Blueprints/Player/BP_PlayerController Object Reference") (DeathIntigator :type "/Game/Blueprints/Player/BP_PlayerController Object Reference"))
  (returns (Spectator :type "/Game/Blueprints/Game/Spectators/BP_GameSpectator Object Reference"))
  (locals (L_Player :type "/Game/Blueprints/Player/BP_PlayerController Object Reference") (L_Intigator :type "/Game/Blueprints/Player/BP_PlayerController Object Reference") (L_Spectator :type "/Game/Blueprints/Game/Spectators/BP_GameSpectator Object Reference"))
  (set `local.L_Player` Player)
  (bind _output_get (set `local.L_Intigator` DeathIntigator))
  (`/Engine/EditorBlueprintResources/StandardMacros.IsValid` _output_get
    (:`Is Valid`
      (bind _returnvalue (`|SpawnActorFromClass` "/Game/Blueprints/Game/Spectators/BP_GameSpectator-CharFollow.BP_GameSpectator-CharFollow_C" (`self.GetTransform` (`Controller.K2_GetPawn` (`local.L_Intigator`))) "Undefined" "OverrideRootScale" null null (`local.L_Player`) null))
      (set `local.L_Spectator` _returnvalue))
    (:`Is Not Valid`
      (bind _returnvalue_2 (`|SpawnActorFromClass` "/Game/Blueprints/Game/Spectators/BP_GameSpectator_Free.BP_GameSpectator_Free_C" (`self.GetTransform` (`Controller.K2_GetPawn` (`local.L_Player`))) "Undefined" "OverrideRootScale" null (`local.L_Player`) null))
      (set `local.L_Spectator` _returnvalue_2)))
  (`Controller.Possess` (`local.L_Player`) (`local.L_Spectator`))
  (bind _asbp_game_spectator__char_follow (cast `/Game/Blueprints/Game/Spectators/BP_GameSpectator-CharFollow` (`local.L_Spectator`))
    (:`then`
      (set `/Game/Blueprints/Game/Spectators/BP_GameSpectator-CharFollow.FollowCharacter` (`local.L_Player`) _asbp_game_spectator__char_follow))
    (:`CastFailed`
      _))
  (return (`local.L_Spectator`)))

(fn `StartRound`
  (for _array_element (`GameStateBase.PlayerArray` (`GameplayStatics.GetGameState`))
    (bind _asbp_player_controller (cast `/Game/Blueprints/Player/BP_PlayerController` (`self.GetOwner` _array_element)))
    (`self.SpawnPlayer` _asbp_player_controller))
  (`self.RoundStarted`))

(fn `StopRound`
  (params (StopReason :type String))
  (for _array_element (`GameStateBase.PlayerArray` (`GameplayStatics.GetGameState`))
    (bind _asbp_player_controller (cast `/Game/Blueprints/Player/BP_PlayerController` (`self.GetOwner` _array_element)))
    (`self.SpawnSpectator` _asbp_player_controller))
  (`self.RoundEnded` StopReason))

(fn `TimeLimitReched`
  (if (`self.LimitByTime`)
    (`self.StopRound` "")))

(fn `UpdateDeathPoints`
  (params (Character :type "/Game/Blueprints/Player/BP_PlayerController Object Reference") (Instigator :type "/Game/Blueprints/Player/BP_PlayerController Object Reference"))
  (`/Game/Blueprints/Player/BP_PlayerState.AddDeath` (cast `/Game/Blueprints/Player/BP_PlayerState` (`Controller.PlayerState` Character) :!pure true))
  (`/Game/Blueprints/Player/BP_PlayerState.AddKill` (cast `/Game/Blueprints/Player/BP_PlayerState` (`Controller.PlayerState` Instigator) :!pure true)))

(fn `UserConstructionScript`)
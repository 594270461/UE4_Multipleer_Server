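; Base game state that tracks whether a round is in progress and how long it has run.
; On the server it binds to BP_BaseGameMode's round start and end events, setting a replicated RoundInProgress flag and multicasting the end reason.
; The flag's RepNotify fires RoundStarted and starts or clears a one-second server timer.
; Each tick advances RoundTime and fires TimeEnded once the game mode's TimeLimit is reached.
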(event `self.ReceiveTick`
  (params (DeltaSeconds :type "Float (single-precision)")))

(event `OnRoundEnded`
  (params (Reason :type String))
  (`self.MulticastRoundEnd` Reason)
  (set `self.RoundInProgress` false))

(event `MulticastRoundEnd`
  (params (Reason :type String))
  (`self.RoundEnded` Reason))

(event `OnRoundStarted`
  (set `self.RoundInProgress` true))

(event `self.ReceiveBeginPlay`
  (`/Engine/EditorBlueprintResources/ActorMacros.Switch Has Authority`
    (:`Authority`
      (add `/Game/Blueprints/Game/BP_BaseGameMode.RoundEnded` (cast `/Game/Blueprints/Game/BP_BaseGameMode` (`GameplayStatics.GetGameMode`) :!pure true) (delegate `OnRoundEnded`))
      (add `/Game/Blueprints/Game/BP_BaseGameMode.RoundStarted` (cast `/Game/Blueprints/Game/BP_BaseGameMode` (`GameplayStatics.GetGameMode`) :!pure true) (delegate `OnRoundStarted`)))))

(fn `GetRoundTime`
  (returns (Minutes :type Integer) (Seconds :type Integer))
  (return (`self.CurrentMinute`) (`self.CurrentSeconds`)))

(fn `OnRep_RoundInProgress`
  (if (`self.RoundInProgress`)
    (`self.RoundStarted`)
    (`/Engine/EditorBlueprintResources/ActorMacros.Switch Has Authority`
      (:`Authority`
        (`self.StartRoundTimer`)))
    (else
      (`/Engine/EditorBlueprintResources/ActorMacros.Switch Has Authority`
        (:`Authority`
          (`KismetSystemLibrary.K2_ClearAndInvalidateTimerHandle` (`self.TimeTickTimer`)))))))

(fn `RoundTimeTick`
  (bind _output_get (set `self.RoundTime` (+ (`self.RoundTime`) (`KismetMathLibrary.MakeTimespan` 0 0 0 1))))
  (bind (_days _hours _minutes _seconds) (`KismetMathLibrary.BreakTimespan` _output_get))
  (set `self.CurrentMinute` _minutes)
  (set `self.CurrentSeconds` _seconds)
  (if (and (>= (`self.RoundTime`) (`/Game/Blueprints/Game/BP_BaseGameMode.TimeLimit` (cast `/Game/Blueprints/Game/BP_BaseGameMode` (`GameplayStatics.GetGameMode`) :!pure true))) (`self.RoundInProgress`))
    (`self.TimeEnded`)))

(fn `StartRoundTimer`
  (bind _returnvalue (`KismetSystemLibrary.K2_SetTimer` null "RoundTimeTick" 1.0 true))
  (set `self.TimeTickTimer` _returnvalue))

(fn `UserConstructionScript`)
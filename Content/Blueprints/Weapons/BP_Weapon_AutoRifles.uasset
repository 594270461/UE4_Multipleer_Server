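; Auto rifle weapon Blueprint that shows its ammo on a TextRender component.
; The text is set to current over total ammo on BeginPlay and refreshed whenever the replicated CurrentAmmo triggers its OnRep event.
; UseWeapon, StopRateDelay and the construction script only call their parent versions, so firing logic is left to the parent class.
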(event `self.StopRateDelay`
  (`parent.StopRateDelay`))

(event `self.ReceiveBeginPlay`
  (`TextRenderComponent.K2_SetText` (`self.TextRender`) (`|FormatText` "{A} / {B}" (`self.CurrentAmmo`) (`self.TotalAmmo`)) :!label _label))

(event `self.OnRep_CurrentAmmo`
  (goto _label))

(fn `UserConstructionScript`
  (`parent.UserConstructionScript`))

(fn `UseWeapon`
  (returns (Used :type Boolean))
  (bind _used (`parent.UseWeapon`))
  (return _used))
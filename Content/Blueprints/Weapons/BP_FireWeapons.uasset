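; Firearm weapon Blueprint that extends a parent weapon with shooting, ammo checks and timed reloading.
; UseWeapon spawns FireProjectile if that class is set, otherwise applies point damage via a debug-drawn line trace; both start at the player camera along the owner's forward vector.
; Reload, or firing on empty with reserve ammo, sets Reloading, whose RepNotify runs the reload timer on authority, using class-default CurrentAmmo as magazine size.
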(event `Debug_DrawSeverTrace`
  (params (Start :type "Vector Structure") (End :type "Vector Structure") (Hit :type "Vector Structure"))
  (`KismetSystemLibrary.DrawDebugLine` Start End (struct :`R` 0.037938 :`G` 1.0 :`B` 0.094347 :`A` 1.0) 5.0 2.0)
  (`KismetSystemLibrary.DrawDebugSphere` Hit 40.0 8 (struct :`R` 1.0 :`G` 0.209795 :`A` 1.0) 5.0 2.0))

(event `self.StopRateDelay`
  (`parent.StopRateDelay`))

(fn `AbleToReload`
  (returns (ReturnValue :type Boolean))
  (return (and (!= (`.CurrentAmmo` (defaults `/Game/Blueprints/Weapons/BP_FireWeapons` (`GameplayStatics.GetObjectClass` self))) (`self.CurrentAmmo`)) (> (`self.TotalAmmo`) 0) (not (`KismetSystemLibrary.K2_IsValidTimerHandle` (`self.ReloadTimer`))))))

(fn `AbleToUseWeapon`
  (returns (Out :type Boolean))
  (return (and (`parent.AbleToUseWeapon`) (not (`self.Reloading`)))))

(fn `GetFireTrace`
  (returns (Hit :type "HitResult Structure"))
  (bind _asbp_player_character (cast `/Game/Blueprints/Player/BP_PlayerCharacter` (`self.GetInstigator`)))
  (bind _returnvalue (`SceneComponent.K2_GetComponentLocation` (`/Game/Blueprints/Player/BP_PlayerCharacter.Camera` _asbp_player_character)))
  (bind _outhit (`KismetSystemLibrary.LineTraceSingleForObjects` _returnvalue (+ _returnvalue (* (`self.GetActorForwardVector` (`self.GetOwner`)) 10000)) (`|MakeArray` "ObjectTypeQuery2" "ObjectTypeQuery1" "ObjectTypeQuery3" :!type "EObjectTypeQuery Enum") false (`|MakeArray` (`self.GetInstigator`) :!type "Actor Object Reference")))
  (bind (_bblockinghit _binitialoverlap _time _distance _location _impactpoint _normal _impactnormal _physmat _hitactor _hitcomponent _hitbonename _hititem _faceindex _tracestart _traceend) (`GameplayStatics.BreakHitResult` _outhit))
  (`self.Debug_DrawSeverTrace` _tracestart _traceend _location)
  (return _outhit))

(fn `OnRep_Reloading`
  (`/Engine/EditorBlueprintResources/ActorMacros.Switch Has Authority`
    (:`Authority`
      (if (`self.Reloading`)
        (if (`self.AbleToReload`)
          (`KismetSystemLibrary.PrintString` "Reloading" true true (struct :`G` 0.004274 :`B` 1.0 :`A` 1.0))
          (bind _returnvalue (`KismetSystemLibrary.K2_SetTimer` null "ReloadFinished" (`self.ReloadTime`)))
          (set `self.ReloadTimer` _returnvalue)
          (set `self.AmmoToReload` (`KismetMathLibrary.Min` (- (defaults `/Game/Blueprints/Weapons/BP_FireWeapons` (`GameplayStatics.GetObjectClass` self)) (`self.CurrentAmmo`)) (`self.TotalAmmo`)))
          (else
            (set `self.Reloading` false)
            (`KismetSystemLibrary.PrintString` "Not able to relaod" true true (struct :`R` 1.0 :`G` 0.154102 :`A` 1.0))))))))

(fn `Reload`
  (set `self.Reloading` true))

(fn `ReloadFinished`
  (set `self.Reloading` false)
  (set `self.CurrentAmmo` (+ (`self.AmmoToReload`) (`self.AmmoToReload`)))
  (set `self.TotalAmmo` (- (`self.TotalAmmo`) (`self.AmmoToReload`)))
  (`KismetSystemLibrary.K2_ClearAndInvalidateTimerHandle` (`self.ReloadTimer`)))

(fn `SpawnShootProjectile`
  (bind _asbp_player_character (cast `/Game/Blueprints/Player/BP_PlayerCharacter` (`self.GetInstigator`)))
  (`|SpawnActorFromClass` (`self.FireProjectile`) (`KismetMathLibrary.MakeTransform` (+ (`SceneComponent.K2_GetComponentLocation` (`/Game/Blueprints/Player/BP_PlayerCharacter.Camera` _asbp_player_character)) (* (`self.GetActorForwardVector` (`self.GetOwner`)) 50)) (`KismetMathLibrary.Conv_VectorToRotator` (`self.GetActorForwardVector` (`self.GetOwner`)))) "Undefined" "OverrideRootScale" self (`self.Damage`) (`self.GetInstigator`)))

(fn `UserConstructionScript`
  (`parent.UserConstructionScript`))

(fn `UseWeapon`
  (returns (Used :type Boolean))
  (bind _used (`parent.UseWeapon`))
  (`KismetSystemLibrary.PrintString` (`KismetStringLibrary.Concat_StrStr` (`KismetStringLibrary.Conv_IntToString` (`self.CurrentAmmo`)) " | " (`KismetStringLibrary.Conv_IntToString` (`self.TotalAmmo`))) true true (struct :`R` 0.05725 :`B` 1.0 :`A` 1.0) 1.0)
  (if _used
    (if (`KismetSystemLibrary.IsValidClass` (`self.FireProjectile`))
      (`self.SpawnShootProjectile`)
      (return true)
      (else
        (bind _hit (`self.GetFireTrace`))
        (bind (_bblockinghit _binitialoverlap _time _distance _location _impactpoint _normal _impactnormal _physmat _hitactor _hitcomponent _hitbonename _hititem _faceindex _tracestart _traceend) (`GameplayStatics.BreakHitResult` _hit))
        (`GameplayStatics.ApplyPointDamage` _hitactor (`self.Damage`) (`KismetMathLibrary.GetDirectionUnitVector` _traceend _tracestart) _hit (`self.GetInstigatorController`) self)
        (return true)))
    (elif (and (<= (`self.CurrentAmmo`) 0) (> (`self.TotalAmmo`) 0))
      (set `self.Reloading` true)
      (return false)
      (else
        (return false)))))
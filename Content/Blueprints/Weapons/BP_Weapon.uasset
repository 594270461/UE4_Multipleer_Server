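; Replicated weapon actor that players pick up through Interact, which hands it to their BPWeaponManager.
; UseWeapon spends ammo and starts a rate-limit timer, whose callback re-fires while AutoFire is held active.
; OnRep_WeaponOwner handles equip and drop: authority attaches to the owner actor, while remotes attach the current weapon to the visible mesh's GripPoint or hide it.
; Clearing the owner detaches, reveals and moves it to DropWeaponLocation.
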(fn `AbleToUseWeapon`
  (returns (Out :type Boolean))
  (return (and (not (`self.UseFreezedByRate`)) (> (`self.CurrentAmmo`) 0))))

(fn `Interact`
  (params (PlayerCharacter :type "/Game/Blueprints/Player/BP_PlayerCharacter Object Reference"))
  (returns (Success :type Boolean))
  (`/Game/Blueprints/Components/Player/BP_WeaponManager.AddWeapon` (`/Game/Blueprints/Player/BP_PlayerCharacter.BP_WeaponManager` PlayerCharacter) self)
  (return false))

(fn `OnRep_CurrentAmmo`)

(fn `OnRep_WeaponOwner`
  (locals (L_WeaponOwner :type "/Game/Blueprints/Player/BP_PlayerCharacter Object Reference"))
  (bind _weaponowner (`self.WeaponOwner`)
    (:`then`
      (bind _output_get (set `local.L_WeaponOwner` _weaponowner))
      (bind _output_get_2 (set `self.Instigator` _output_get))
      (`self.SetOwner` (`Pawn.GetController` _output_get_2))
      (`self.SetActorEnableCollision` false)
      (`/Engine/EditorBlueprintResources/ActorMacros.Switch Has Authority`
        (:`Authority`
          (`self.K2_AttachToActor` (`local.L_WeaponOwner`) "None" "SnapToTarget" "SnapToTarget" "SnapToTarget"))
        (:`Remote`
          (if (not (== (`/Game/Blueprints/Components/Player/BP_WeaponManager.CurrentWeapon` (`/Game/Blueprints/Player/BP_PlayerCharacter.BP_WeaponManager` (`self.WeaponOwner`))) self))
            (`self.SetActorHiddenInGame` true)
            (else
              (`self.K2_AttachToComponent` self (`/Game/Blueprints/Player/BP_PlayerCharacter.GetVisibleMesh` (`self.WeaponOwner`)) "GripPoint" "SnapToTarget" "SnapToTarget" "SnapToTarget" true))))))
    (:`else`
      (`self.K2_DetachFromActor` "KeepRelative")
      (`self.SetActorHiddenInGame` false)
      (`self.SetActorEnableCollision` true)
      (`self.K2_SetActorLocation` (`self.DropWeaponLocation`) false true)
      (set `self.Instigator` null)
      (`self.SetOwner` null))))

(fn `SetWeaponOwner`
  (params (PlayerCharacter :type "/Game/Blueprints/Player/BP_PlayerCharacter Object Reference")))

(fn `StopRateDelay`
  (set `self.UseFreezedByRate` false)
  (if (and (`self.AutoFire`) (`self.FireActive`))
    (`self.UseWeapon`)))

(fn `StopUseWeapon`
  (set `self.FireActive` false))

(fn `UserConstructionScript`)

(fn `UseWeapon`
  (returns (Used :type Boolean))
  (if (`self.AbleToUseWeapon`)
    (`/Engine/EditorBlueprintResources/StandardMacros.DecrementInt` (`self.CurrentAmmo`)
      (:`  `
        (`KismetSystemLibrary.K2_SetTimer` null "StopRateDelay" (`self.UseRate`))
        (set `self.UseFreezedByRate` true)
        (if (`self.AutoFire`)
          (set `self.FireActive` true))
        (return true)))
    (else
      (set `self.FireActive` false)
      (return false))))